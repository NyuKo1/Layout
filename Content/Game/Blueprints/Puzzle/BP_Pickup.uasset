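; BP_Pickup is a puzzle item that unlocks a linked door and/or button when the player collects it.
; On BeginPlay it tints the item through a dynamic material instance and its glow light, both using ItemColor.
; When the player pawn overlaps the trigger, it calls Unlock on any valid linked DoorToUnlock and ButtonToUnlock, prints PickupMessage in the item colour, and destroys itself.
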(event `self.ReceiveBeginPlay`
  ;[0.1 0.35 0.8] 1. SETUP - colour the item and its glow with ItemColor
  (bind _returnvalue (`PrimitiveComponent.CreateDynamicMaterialInstance` (`self.Item`) 0 null "None"))
  (set `self.ItemMID` _returnvalue)
  (`MaterialInstanceDynamic.SetVectorParameterValue` (`self.ItemMID`) "Color" (`self.ItemColor`))
  (`LightComponent.SetLightColor` (`self.Glow`) (`self.ItemColor`) true))

(event `self.Trigger.OnComponentBeginOverlap`
  (params (OverlappedComponent :type "PrimitiveComponent Object Reference") (OtherActor :type "Actor Object Reference") (OtherComp :type "PrimitiveComponent Object Reference") (OtherBodyIndex :type Integer) (bFromSweep :type Boolean) (SweepResult :type "HitResult Structure (by ref)"))
  ;[0.1 0.55 0.25] 2. PICK UP - unlock the linked DoorToUnlock and/or ButtonToUnlock, show PickupMessage, remove the item
  (if (== OtherActor (`GameplayStatics.GetPlayerPawn` 0))
    (if (`KismetSystemLibrary.IsValid` (`self.DoorToUnlock`))
      (`/Game/Game/Blueprints/Interactables/BP_HingedDoor.Unlock` (`self.DoorToUnlock`)))
    (if (`KismetSystemLibrary.IsValid` (`self.ButtonToUnlock`))
      (`/Game/Game/Blueprints/Interactables/BP_ElevatorButton.Unlock` (`self.ButtonToUnlock`)))
    (`KismetSystemLibrary.PrintString` (`self.PickupMessage`) true true (`self.ItemColor`) 5.0 "Quest")
    (`self.K2_DestroyActor`)))

(fn `UserConstructionScript`)