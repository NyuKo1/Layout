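; BP_QuestMessage is a trigger zone that shows a configurable message on screen when the player enters it.
; The Trigger component's begin-overlap event accepts only player pawn 0, then displays Message through Print String with a configurable color and duration, with no UI widget involved.
; When OnlyOnce is set, the AlreadyShown flag suppresses repeat displays.
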(event `self.Trigger.OnComponentBeginOverlap`
  (params (OverlappedComponent :type "PrimitiveComponent Object Reference") (OtherActor :type "Actor Object Reference") (OtherComp :type "PrimitiveComponent Object Reference") (OtherBodyIndex :type Integer) (bFromSweep :type Boolean) (SweepResult :type "HitResult Structure (by ref)"))
  ;[0.1 0.35 0.8] PLAYER ENTERS THE ZONE - show the Message on screen (only once if OnlyOnce)
  (if (== OtherActor (`GameplayStatics.GetPlayerPawn` 0))
    (if (not (and (`self.OnlyOnce`) (`self.AlreadyShown`)))
      (set `self.AlreadyShown` true)
      (`KismetSystemLibrary.PrintString` (`self.Message`) true true (`self.TextColor`) (`self.Duration`) "Quest"))))

(fn `UserConstructionScript`)