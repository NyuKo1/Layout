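; BP_TrapZone is a lava trap that sends the player back to a respawn point on contact.
; On BeginPlay it creates a dynamic material for the lava mesh and tints it and its light with TrapColor.
; When player pawn 0 overlaps the Trigger and RespawnPoint is valid, it prints a warning message in that color and teleports the pawn to that actor's location and rotation.
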(event `self.ReceiveBeginPlay`
  ;[0.1 0.35 0.8] 1. SETUP - lava colour
  (bind _returnvalue (`PrimitiveComponent.CreateDynamicMaterialInstance` (`self.Lava`) 0 null "None"))
  (set `self.LavaMID` _returnvalue)
  (`MaterialInstanceDynamic.SetVectorParameterValue` (`self.LavaMID`) "Color" (`self.TrapColor`))
  (`LightComponent.SetLightColor` (`self.LavaLight`) (`self.TrapColor`) true))

(event `self.Trigger.OnComponentBeginOverlap`
  (params (OverlappedComponent :type "PrimitiveComponent Object Reference") (OtherActor :type "Actor Object Reference") (OtherComp :type "PrimitiveComponent Object Reference") (OtherBodyIndex :type Integer) (bFromSweep :type Boolean) (SweepResult :type "HitResult Structure (by ref)"))
  ;[0.1 0.55 0.25] 2. TOUCH THE LAVA - warn the player and teleport them back to RespawnPoint
  (if (== OtherActor (`GameplayStatics.GetPlayerPawn` 0))
    (if (`KismetSystemLibrary.IsValid` (`self.RespawnPoint`))
      (`KismetSystemLibrary.PrintString` (`self.Message`) true true (`self.TrapColor`) 3.0 "Hint")
      (`self.K2_TeleportTo` OtherActor (`self.K2_GetActorLocation` (`self.RespawnPoint`)) (`self.K2_GetActorRotation` (`self.RespawnPoint`))))))

(fn `UserConstructionScript`)