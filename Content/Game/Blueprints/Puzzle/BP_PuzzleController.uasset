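; Puzzle controller that opens a secret door once all of its linked rotating pillars show their correct symbols.
; An orb and its light start in the unsolved color through a dynamic material instance.
; CheckSolution scans every BP_RotatingPillar assigned to this controller and compares its current index to the correct one.
; When all match, it latches as solved, recolors orb and light, opens the SecretDoor if valid and prints a message.
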(event `self.ReceiveBeginPlay`
  ;[0.1 0.35 0.8] 1. SETUP - orb glows red (unsolved)
  (bind _returnvalue (`PrimitiveComponent.CreateDynamicMaterialInstance` (`self.Orb`) 0 null "None"))
  (set `self.OrbMID` _returnvalue)
  (`MaterialInstanceDynamic.SetVectorParameterValue` (`self.OrbMID`) "Color" (`self.ColorUnsolved`))
  (`LightComponent.SetLightColor` (`self.OrbLight`) (`self.ColorUnsolved`) true))

(event `CheckSolution`
  ;[0.1 0.55 0.25] 2. CheckSolution - every pillar linked to me must show its CorrectIndex. All correct -> solved, orb turns green, open the SecretDoor
  (if (not (`self.Solved`))
    (set `self.AllCorrect` true)
    (bind _outactors (`GameplayStatics.GetAllActorsOfClass` "/Game/Game/Blueprints/Puzzle/BP_RotatingPillar.BP_RotatingPillar_C"))
    (for _array_element _outactors
      (if (and (== (`/Game/Game/Blueprints/Puzzle/BP_RotatingPillar.Controller` _array_element) self) (!= (`/Game/Game/Blueprints/Puzzle/BP_RotatingPillar.CurrentIndex` _array_element) (`/Game/Game/Blueprints/Puzzle/BP_RotatingPillar.CorrectIndex` _array_element)))
        (set `self.AllCorrect` false)))
    (if (`self.AllCorrect`)
      (set `self.Solved` true)
      (`MaterialInstanceDynamic.SetVectorParameterValue` (`self.OrbMID`) "Color" (`self.ColorSolved`))
      (`LightComponent.SetLightColor` (`self.OrbLight`) (`self.ColorSolved`) true)
      (if (`KismetSystemLibrary.IsValid` (`self.SecretDoor`))
        (`/Game/Game/Blueprints/Interactables/BP_SlidingDoor.Open` (`self.SecretDoor`)))
      (`KismetSystemLibrary.PrintString` "The symbols align... a SECRET PASSAGE opens!" true true (struct :`R` 0.3 :`G` 1.0 :`B` 0.5 :`A` 1.0) 6.0 "Quest"))))

(fn `UserConstructionScript`)