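; BP_RotatingPillar is a puzzle pillar with a coloured symbol that the player turns through four directions.
; Overlapping InteractZone enables its input, so each IA_Interact press advances CurrentIndex, adds 90 degrees to TargetYaw and asks the Controller to check the solution immediately.
; Tick turns Pivot toward the ever-increasing TargetYaw at constant speed, so the index wraps while rotation keeps going the same way.
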(event `self.ReceiveBeginPlay`
  ;[0.1 0.35 0.8] 1. SETUP - colour the symbol, face the starting direction (CurrentIndex x 90 deg)
  (bind _returnvalue (`PrimitiveComponent.CreateDynamicMaterialInstance` (`self.Symbol`) 0 null "None"))
  (set `self.SymbolMID` _returnvalue)
  (`MaterialInstanceDynamic.SetVectorParameterValue` (`self.SymbolMID`) "Color" (`self.SymbolColor`))
  (set `self.TargetYaw` (`KismetMathLibrary.Conv_IntToDouble` (* (`self.CurrentIndex`) 90)))
  (set `self.VisualYaw` (`self.TargetYaw`)))

(event `self.ReceiveTick`
  (params (DeltaSeconds :type "Float (single-precision)"))
  ;[0.1 0.55 0.25] 5. EVERY FRAME - rotate smoothly toward TargetYaw
  (set `self.VisualYaw` (`KismetMathLibrary.FInterpTo_Constant` (`self.VisualYaw`) (`self.TargetYaw`) DeltaSeconds (`self.TurnSpeed`)))
  (`SceneComponent.K2_SetRelativeRotation` (`self.Pivot`) (`KismetMathLibrary.MakeRotator` 0.0 0.0 (`self.VisualYaw`)) false false))

(event `self.InteractZone.OnComponentBeginOverlap`
  (params (OverlappedComponent :type "PrimitiveComponent Object Reference") (OtherActor :type "Actor Object Reference") (OtherComp :type "PrimitiveComponent Object Reference") (OtherBodyIndex :type Integer) (bFromSweep :type Boolean) (SweepResult :type "HitResult Structure (by ref)"))
  ;[0.65 0.35 0.05] 2. Player nearby -> listen to the E key
  (if (== OtherActor (`GameplayStatics.GetPlayerPawn` 0))
    (`self.EnableInput` (`GameplayStatics.GetPlayerController` 0))))

(event `self.InteractZone.OnComponentEndOverlap`
  (params (OverlappedComponent :type "PrimitiveComponent Object Reference") (OtherActor :type "Actor Object Reference") (OtherComp :type "PrimitiveComponent Object Reference") (OtherBodyIndex :type Integer))
  ;[0.5 0.15 0.6] 3. Player left -> stop listening
  (if (== OtherActor (`GameplayStatics.GetPlayerPawn` 0))
    (`self.DisableInput` (`GameplayStatics.GetPlayerController` 0))))

(event `EnhancedInput|/Game/Input/Actions/IA_Interact`
  (params (ActionValue :type Boolean) (ElapsedSeconds :type "Float (double-precision)") (TriggeredSeconds :type "Float (double-precision)") (InputAction :type "InputAction Object Reference" :default "/Game/Input/Actions/IA_Interact.IA_Interact"))
  ;[0.1 0.5 0.55] 4. E PRESSED - turn to the next direction (0-3) and ask the Controller to check the puzzle
  (:`Started`
    (set `self.CurrentIndex` (mod (+ (`self.CurrentIndex`) 1) 4))
    (set `self.TargetYaw` (+ (`self.TargetYaw`) 90.0))
    (if (`KismetSystemLibrary.IsValid` (`self.Controller`))
      (`/Game/Game/Blueprints/Puzzle/BP_PuzzleController.CheckSolution` (`self.Controller`)))))

(fn `UserConstructionScript`)