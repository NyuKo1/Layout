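; A two-panel sliding door for one elevator floor, opening when the elevator arrives there and closing when it departs.
; Tick eases a shared offset at constant speed to slide the panels apart or together.
; Optional auto-close waits after arrival, rechecking every second while the player stands in the doorway.
; A dynamic material lamp and status light show open or closed color, and BeginPlay syncs to the elevator's current floor.
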(event `self.ReceiveBeginPlay`
  ;[0.1 0.35 0.8] 1. SETUP - remember where both panels sit when closed, make the lamp material, start closed (open if the elevator is already here)
  (set `self.LeftClosed` (`SceneComponent.RelativeLocation` (`self.DoorLeft`)))
  (set `self.RightClosed` (`SceneComponent.RelativeLocation` (`self.DoorRight`)))
  (bind _returnvalue (`PrimitiveComponent.CreateDynamicMaterialInstance` (`self.StatusLamp`) 0 null "None"))
  (set `self.LampMID` _returnvalue)
  (`self.Close`)
  (if (`KismetSystemLibrary.IsValid` (`self.Elevator`))
    (`self.HandleArrived` (`/Game/Game/Blueprints/BP_MovingPlatform.CurrentFloor` (`self.Elevator`)))))

(event `self.ReceiveTick`
  (params (DeltaSeconds :type "Float (single-precision)"))
  (bind _returnvalue (`KismetMathLibrary.MakeVector` 0.0 (`self.OpenAmount`)))
  ;[0.1 0.55 0.25] 2. MOVEMENT (every frame) - ease OpenAmount toward SlideDistance (open) or 0 (closed) at OpenSpeed, slide the left panel left and the right panel right by OpenAmount
  (set `self.OpenAmount` (`KismetMathLibrary.FInterpTo_Constant` (`self.OpenAmount`) (`KismetMathLibrary.SelectFloat` (`self.SlideDistance`) 0.0 (`self.IsOpen`)) DeltaSeconds (`self.OpenSpeed`)))
  (`SceneComponent.K2_SetRelativeLocation` (`self.DoorLeft`) (- (`self.LeftClosed`) _returnvalue) false false)
  (`SceneComponent.K2_SetRelativeLocation` (`self.DoorRight`) (+ (`self.RightClosed`) _returnvalue) false false))

(event `SetLamp`
  (params (Color :type "LinearColor Structure"))
  ;[0.65 0.35 0.05] 8. SetLamp(Color) - paint the lamp and the status light
  (`MaterialInstanceDynamic.SetVectorParameterValue` (`self.LampMID`) "Color" Color)
  (`LightComponent.SetLightColor` (`self.StatusLight`) Color true))

(event `TryAutoClose`
  ;[0.5 0.15 0.6] 5. TryAutoClose - still open? player in DoorwayZone -> check again in 1 s, otherwise Close
  (if (`self.IsOpen`)
    (if (`PrimitiveComponent.IsOverlappingActor` (`self.DoorwayZone`) (`GameplayStatics.GetPlayerPawn` 0))
      (`KismetSystemLibrary.RetriggerableDelay` 1.0)
      (`self.TryAutoClose`)
      (else
        (`self.Close`)))))

(event `Open`
  ;[0.1 0.5 0.55] 6. Open - target = open, lamp GREEN
  (set `self.IsOpen` true)
  (`self.SetLamp` (`self.ColorOpen`)))

(event `Close`
  ;[0.6 0.15 0.15] 7. Close - target = closed, lamp RED
  (set `self.IsOpen` false)
  (`self.SetLamp` (`self.ColorClosed`)))

(event `HandleDeparted`
  (params (DestinationFloor :type Integer))
  ;[0.1 0.35 0.8] 4. Message from elevator: leaving -> Close
  (`self.Close`))

(event `HandleArrived`
  (params (ArrivedFloor :type Integer))
  ;[0.1 0.55 0.25] 3. Message from elevator: arrived. My floor -> Open, then after AutoCloseDelay try to close
  (if (== ArrivedFloor (`self.Floor`))
    (`self.Open`)
    (if (`self.AutoClose`)
      (`KismetSystemLibrary.RetriggerableDelay` (`self.AutoCloseDelay`))
      (`self.TryAutoClose`))))

(fn `UserConstructionScript`)