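; Hinged door that the player pushes open by walking into it, lockable until the key pickup calls Unlock.
; Each Tick swings it with damping and optional spring self-closing, rotates it clear of the player capsule, then clamps the angle.
; The push is computed in hinge space without physics and becomes swing momentum, while an unlocked door ignores Pawn collision.
; The lock state also colors lamp and light, and the Construction Script sizes door and frame.
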(event `self.ReceiveBeginPlay`
  ;[0.1 0.35 0.8] SETUP - lock lamp material, apply the lock state
  (bind _returnvalue (`PrimitiveComponent.CreateDynamicMaterialInstance` (`self.LockLamp`) 0 null "None"))
  (set `self.LockMID` _returnvalue)
  (`self.ApplyLockState`))

(event `self.ReceiveTick`
  (params (DeltaSeconds :type "Float (single-precision)"))
  ;[0.1 0.55 0.25] EVERY FRAME - store the frame time (Dt), then run the three steps below in order
  (set `self.Dt` (`KismetMathLibrary.FMax` DeltaSeconds 0.001))
  (`self.FreeSwing`)
  (`self.PushByPlayer`)
  (`self.ApplyLimits`))

(event `ApplyLockState`
  ;[0.65 0.35 0.05] LOCK STATE - locked: door is solid + red lamp, unlocked: door can be pushed + green lamp
  (if (`self.Locked`)
    (`PrimitiveComponent.SetCollisionProfileName` (`self.Door`) "BlockAll" true)
    (`MaterialInstanceDynamic.SetVectorParameterValue` (`self.LockMID`) "Color" (`self.ColorLocked`))
    (`LightComponent.SetLightColor` (`self.LockLight`) (`self.ColorLocked`) true)
    (else
      (`PrimitiveComponent.SetCollisionProfileName` (`self.Door`) "IgnoreOnlyPawn" true)
      (`MaterialInstanceDynamic.SetVectorParameterValue` (`self.LockMID`) "Color" (`self.ColorUnlocked`))
      (`LightComponent.SetLightColor` (`self.LockLight`) (`self.ColorUnlocked`) true))))

(event `FreeSwing`
  ;[0.5 0.15 0.6] STEP 1  FreeSwing - the door keeps its momentum: spring pulls it back to 0 deg if SelfClosing, SwingDamping slows it, then CurrentAngle moves by AngularVelocity
  (set `self.PrevAngle` (`self.CurrentAngle`))
  (set `self.AngularVelocity` (* (+ (`self.AngularVelocity`) (* (`KismetMathLibrary.SelectFloat` (* (* (`self.SwingStiffness`) (`self.CurrentAngle`)) -1.0) 0.0 (`self.SelfClosing`)) (`self.Dt`))) (`KismetMathLibrary.FMax` (- 1.0 (* (`self.SwingDamping`) (`self.Dt`))))))
  (set `self.CurrentAngle` (+ (`self.CurrentAngle`) (* (`self.AngularVelocity`) (`self.Dt`)))))

(event `Unlock`
  ;[0.1 0.5 0.55] Unlock - called by the KEY pickup
  (set `self.Locked` false)
  (`self.ApplyLockState`))

(event `ApplyLimits`
  ;[0.6 0.15 0.15] STEP 3  ApplyLimits - keep the angle within +-MaxOpenAngle (stop dead at the limit) and rotate HingePivot
  (if (!= (`self.CurrentAngle`) (`KismetMathLibrary.FClamp` (`self.CurrentAngle`) (* (`self.MaxOpenAngle`) -1.0) (`self.MaxOpenAngle`)))
    (set `self.CurrentAngle` (`KismetMathLibrary.FClamp` (`self.CurrentAngle`) (* (`self.MaxOpenAngle`) -1.0) (`self.MaxOpenAngle`)))
    (set `self.AngularVelocity` 0.0))
  (`SceneComponent.K2_SetRelativeRotation` (`self.HingePivot`) (`KismetMathLibrary.MakeRotator` 0.0 0.0 (`self.CurrentAngle`)) false false))

(event `PushByPlayer`
  ;[0.1 0.35 0.8] STEP 2  PushByPlayer - where is the player, measured from the hinge? If their capsule touches the door, rotate the door just far enough to clear the body and take that push speed as the new AngularVelocity
  (if (`self.Locked`)
    _
    (elif (`KismetSystemLibrary.IsValid` (`GameplayStatics.GetPlayerCharacter` 0))
      (set `self.PlayerRadius` (`CapsuleComponent.GetScaledCapsuleRadius` (`Character.CapsuleComponent` (`GameplayStatics.GetPlayerCharacter` 0))))
      (set `self.PlayerHalfHeight` (`CapsuleComponent.GetScaledCapsuleHalfHeight` (`Character.CapsuleComponent` (`GameplayStatics.GetPlayerCharacter` 0))))
      (set `self.PlayerLocal` (- (`KismetMathLibrary.InverseTransformLocation` (`self.GetTransform`) (`self.K2_GetActorLocation` (`GameplayStatics.GetPlayerCharacter` 0))) (`SceneComponent.RelativeLocation` (`self.HingePivot`))))
      (set `self.PlayerAngle` (`KismetMathLibrary.DegAtan2` (.y (`self.PlayerLocal`)) (.x (`self.PlayerLocal`))))
      (set `self.AngleToDoor` (`KismetMathLibrary.NormalizeAxis` (- (- (`self.PlayerAngle`) 90.0) (`self.CurrentAngle`))))
      (set `self.ClearAngle` (`KismetMathLibrary.DegAsin` (`KismetMathLibrary.FClamp` (/ (+ (+ (`self.PlayerRadius`) (/ (`self.DoorThickness`) 2.0)) (`self.PushMargin`)) (`KismetMathLibrary.FMax` (`KismetMathLibrary.VSizeXY` (`self.PlayerLocal`)) 1.0)))))
      (if (and (and (< (`KismetMathLibrary.VSizeXY` (`self.PlayerLocal`)) (+ (`self.DoorWidth`) (`self.PlayerRadius`))) (and (> (.z (`self.PlayerLocal`)) (* (`self.PlayerHalfHeight`) -1.0)) (< (.z (`self.PlayerLocal`)) (+ (`self.DoorHeight`) (`self.PlayerHalfHeight`))))) (< (`KismetMathLibrary.Abs` (`self.AngleToDoor`)) (`self.ClearAngle`)))
        (set `self.CurrentAngle` (`KismetMathLibrary.NormalizeAxis` (- (- (`self.PlayerAngle`) 90.0) (* (`KismetMathLibrary.SignOfFloat` (`self.AngleToDoor`)) (`self.ClearAngle`)))))
        (set `self.AngularVelocity` (`KismetMathLibrary.FClamp` (/ (- (`self.CurrentAngle`) (`self.PrevAngle`)) (`self.Dt`)) (* (`self.MaxSwingSpeed`) -1.0) (`self.MaxSwingSpeed`)))))))

(fn `UserConstructionScript`
  (bind _returnvalue (+ (`self.DoorHeight`) 10.0))
  (bind _returnvalue_2 (/ (`self.DoorWidth`) 2.0))
  (bind _returnvalue_3 (+ _returnvalue_2 7.0))
  (bind _returnvalue_4 (/ _returnvalue 2.0))
  (bind _returnvalue_5 (`KismetMathLibrary.MakeVector` 0.2 0.1 (/ _returnvalue 100.0)))
  ;[0.1 0.35 0.8] CONSTRUCTION SCRIPT - size and place the door, hinge and frame from DoorWidth / DoorHeight / DoorThickness (runs in the editor whenever you change them)
  (`SceneComponent.K2_SetRelativeLocation` (`self.HingePivot`) (`KismetMathLibrary.MakeVector` 0.0 (* _returnvalue_2 -1.0)) false false)
  (`SceneComponent.K2_SetRelativeLocation` (`self.Door`) (`KismetMathLibrary.MakeVector` 0.0 _returnvalue_2 (+ (/ (`self.DoorHeight`) 2.0) 1.0)) false false)
  (`SceneComponent.SetRelativeScale3D` (`self.Door`) (`KismetMathLibrary.MakeVector` (/ (`self.DoorThickness`) 100.0) (/ (- (`self.DoorWidth`) 2.0) 100.0) (/ (- (`self.DoorHeight`) 2.0) 100.0)))
  (`SceneComponent.K2_SetRelativeLocation` (`self.FrameLeft`) (`KismetMathLibrary.MakeVector` 0.0 (* _returnvalue_3 -1.0) _returnvalue_4) false false)
  (`SceneComponent.SetRelativeScale3D` (`self.FrameLeft`) _returnvalue_5)
  (`SceneComponent.K2_SetRelativeLocation` (`self.FrameRight`) (`KismetMathLibrary.MakeVector` 0.0 _returnvalue_3 _returnvalue_4) false false)
  (`SceneComponent.SetRelativeScale3D` (`self.FrameRight`) _returnvalue_5)
  (`SceneComponent.K2_SetRelativeLocation` (`self.FrameTop`) (`KismetMathLibrary.MakeVector` 0.0 0.0 (+ (`self.DoorHeight`) 5.0)) false false)
  (`SceneComponent.SetRelativeScale3D` (`self.FrameTop`) (`KismetMathLibrary.MakeVector` 0.2 (/ (+ (`self.DoorWidth`) 24.0) 100.0) 0.1)))