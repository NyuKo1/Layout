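; BP_ElevatorButton is an interactable that calls its elevator to the button's floor, unless it is locked until a key card unlocks it.
; An overlap zone enables input for the player, and the interact action triggers the call or prints a locked message.
; A dynamic material and point light share one colour showing locked, floor, moving or arrived state, updated by elevator departure and arrival messages, with a timed arrival highlight.
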(event `self.ReceiveBeginPlay`
  ;[0.1 0.35 0.8] 1. SETUP - make a dynamic material for the glow so its colour can change, then show the starting state
  (bind _returnvalue (`PrimitiveComponent.CreateDynamicMaterialInstance` (`self.ButtonMesh`) 0 null "None"))
  (set `self.IndicatorMID` _returnvalue)
  (`self.RefreshIdleState`))

(event `Unlock`
  ;[0.1 0.55 0.25] Unlock - called by the KEY CARD pickup
  (set `self.Locked` false)
  (`self.RefreshIdleState`))

(event `SetIndicator`
  (params (Color :type "LinearColor Structure"))
  ;[0.65 0.35 0.05] 8. SetIndicator(Color) - paint the button glow and the point light
  (`MaterialInstanceDynamic.SetVectorParameterValue` (`self.IndicatorMID`) "Color" Color)
  (`LightComponent.SetLightColor` (`self.IndicatorLight`) Color true))

(event `RefreshIdleState`
  ;[0.5 0.15 0.6] 7. Idle colour: elevator on my floor -> BLUE, elsewhere -> RED
  (if (`self.Locked`)
    (`self.SetIndicator` (`self.ColorLocked`))
    (elif (`KismetSystemLibrary.IsValid` (`self.Elevator`))
      (if (== (`/Game/Game/Blueprints/Interactables/BP_MovingPlatform.CurrentFloor` (`self.Elevator`)) (`self.Floor`))
        (`self.SetIndicator` (`self.ColorThisFloor`))
        (else
          (`self.SetIndicator` (`self.ColorOtherFloor`)))))))

(event `HandleDeparted`
  (params (DestinationFloor :type Integer))
  ;[0.1 0.5 0.55] 5. Message from elevator: it is leaving -> ORANGE (moving)
  (`self.SetIndicator` (`self.ColorMoving`)))

(event `HandleArrived`
  (params (ArrivedFloor :type Integer))
  ;[0.6 0.15 0.15] 6. Message from elevator: it arrived. My floor -> GREEN, wait ArrivedHighlightTime, then idle colour. Other floor -> RED
  (if (== ArrivedFloor (`self.Floor`))
    (`self.SetIndicator` (`self.ColorArrived`))
    (`KismetSystemLibrary.Delay` (`self.ArrivedHighlightTime`))
    (if (not (`/Game/Game/Blueprints/Interactables/BP_MovingPlatform.IsBusy` (`self.Elevator`)))
      (`self.RefreshIdleState`))
    (else
      (`self.SetIndicator` (`self.ColorOtherFloor`)))))

(event `self.InteractZone.OnComponentBeginOverlap`
  (params (OverlappedComponent :type "PrimitiveComponent Object Reference") (OtherActor :type "Actor Object Reference") (OtherComp :type "PrimitiveComponent Object Reference") (OtherBodyIndex :type Integer) (bFromSweep :type Boolean) (SweepResult :type "HitResult Structure (by ref)"))
  ;[0.1 0.35 0.8] 2. Player walks into InteractZone -> start listening to the E key
  (if (== OtherActor (`GameplayStatics.GetPlayerPawn` 0))
    (`self.EnableInput` (`GameplayStatics.GetPlayerController` 0))))

(event `self.InteractZone.OnComponentEndOverlap`
  (params (OverlappedComponent :type "PrimitiveComponent Object Reference") (OtherActor :type "Actor Object Reference") (OtherComp :type "PrimitiveComponent Object Reference") (OtherBodyIndex :type Integer))
  ;[0.1 0.55 0.25] 3. Player leaves InteractZone -> stop listening to the E key
  (if (== OtherActor (`GameplayStatics.GetPlayerPawn` 0))
    (`self.DisableInput` (`GameplayStatics.GetPlayerController` 0))))

(event `EnhancedInput|/Game/Game/Input/IA_Interact`
  (params (ActionValue :type Boolean) (ElapsedSeconds :type "Float (double-precision)") (TriggeredSeconds :type "Float (double-precision)") (InputAction :type "InputAction Object Reference" :default "/Game/Game/Input/IA_Interact.IA_Interact"))
  ;[0.65 0.35 0.05] 4. E PRESSED - locked: purple + 'needs a key card'. Unlocked: call the elevator to my Floor
  (:`Started`
    (if (`self.Locked`)
      (`KismetSystemLibrary.PrintString` "Locked: this elevator needs a KEY CARD" true true (struct :`R` 0.7 :`G` 0.3 :`B` 1.0 :`A` 1.0) 3.0 "Hint")
      (elif (`KismetSystemLibrary.IsValid` (`self.Elevator`))
        (`/Game/Game/Blueprints/Interactables/BP_MovingPlatform.CallToFloor` (`self.Elevator`) (`self.Floor`))))))

(fn `UserConstructionScript`)